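; BP_Enemy is an enemy that chases the player on sight and takes damage.
; PawnSensing sets a visibility flag, never cleared here, and triggers AI MoveTo toward the player character.
; Tick updates the health bar widget against a 100-point scale and rotates it to face the camera.
; Damage lowers health; the actor is destroyed only by a hit arriving after health is already depleted.
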(event OnSeePawn(PawnSensing)
  (params (Pawn :type Pawn%20Object%20Reference))
  (Variables|Default|SetPlayerVisible true)
  (CallFunction|FollowPlayer))

(event Custom|FollowPlayer
  (if (Variables|Default|GetPlayerVisible)
    (AI|AIMoveTo self "0, 0, 0" (Game|GetPlayerCharacter 0) 5.0 false)))

(event EventBeginPlay)

(event Collision|EventActorBeginOverlap
  (params (OtherActor :type Actor%20Object%20Reference)))

(event EventTick
  (params (DeltaSeconds :type Float%20%28single-precision%29))
  (bind __health_bar_widget (Variables|Default|Get%20Health%20Bar%20Widget))
  (bind _asenemy_health_bar (Utilities|Casting|CastToEnemy_HealthBar (UserInterface|GetWidget (Variables|Default|Get%20Health%20Bar%20Widget))))
  (Progress|SetPercent (Variables|/Game/Enemy/Enemy_HealthBar.Enemy_HealthBar_C|GetHealthBar _asenemy_health_bar) (/ (Variables|Default|GetEnemyHealth) 1e+02))
  (Transformation|SetWorldRotation __health_bar_widget (Math|Rotator|FindLookatRotation (Transformation|GetWorldLocation __health_bar_widget) (Transformation|GetWorldLocation (Variables|/Script/Engine.PlayerCameraManager|GetTransformComponent (Game|GetPlayerCameraManager 0)))) false false))

(event Game|Damage|EventAnyDamage
  (params (Damage :type Float%20%28single-precision%29) (DamageType :type Damage%20Type%20Object%20Reference) (InstigatedBy :type Controller%20Object%20Reference) (DamageCauser :type Actor%20Object%20Reference))
  (if (> (Variables|Default|GetEnemyHealth) 0.0)
    (Variables|Default|SetEnemyHealth (- (Variables|Default|GetEnemyHealth) Damage))
    (else
      (Actor|DestroyActor))))

(fn ConstructionScript)